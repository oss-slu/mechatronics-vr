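; BP_VRHands visualizes the tracked left hand in VR as instanced static meshes, redrawn every tick.
; Each tick clears the instances, gets world-space joint transforms from XR hand tracking, and adds one instance per transform.
; Transforms are built only for valid tracking data with 26 joints, pairing each joint's rotation with the location at index 0, so all instances share one position.
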(event EventBeginPlay)

(event Collision|EventActorBeginOverlap
  (params (OtherActor :type Actor%20Object%20Reference)))

(event EventTick
  (params (DeltaSeconds :type Float%20%28single-precision%29))
  (CallFunction|ClearHands)
  (bind _transforms (CallFunction|GetJointTransforms "Left"))
  (CallFunction|DrawHand _transforms))

(fn ConstructionScript)

(fn GetJointTransforms
  (params (Hand :type EControllerHand%20Enum :default "Left"))
  (bind _newlocalvar (LocalVariables|GetNewLocalVar))
  ;[0 0 0 0.5] Get Actual Hand Tracking Data
  (bind _handtrackingstate (Class|HeadMountedDisplayFunctionLibrary|GetHandTrackingState 0 "UnrealWorldSpace" Hand))
  ;[0.3265 1 0 0.5] Hand Data Validaiton
  (if (.bValid (Utilities|Struct|BreakXRHandTrackingState _handtrackingstate))
    (if (and (== (Utilities|Array|Length (.HandKeyLocations (Utilities|Struct|BreakXRHandTrackingState _handtrackingstate))) 26) (== (Utilities|Array|Length (.HandKeyRotations (Utilities|Struct|BreakXRHandTrackingState _handtrackingstate))) 26))
      ;[0.006052 0.005809 0.15 0.5] Create a joint transform from the join locationsand rotationss
      (for (_ _array_index) (.HandKeyLocations (Utilities|Struct|BreakXRHandTrackingState _handtrackingstate))
        (Utilities|Array|Add _newlocalvar (Math|Transform|MakeTransform (Utilities|Array|Get(acopy) (.HandKeyLocations (Utilities|Struct|BreakXRHandTrackingState _handtrackingstate))) (Class|KismetMathLibrary|QuatRotator (Utilities|Array|Get(acopy) (.HandKeyRotations (Utilities|Struct|BreakXRHandTrackingState _handtrackingstate)) _array_index)))))
      (return _newlocalvar))))

(fn DrawHand
  (params (Transforms :type Array%20of%20Transforms))
  (for _array_element Transforms
    (Components|InstancedStaticMesh|AddInstance (Variables|Default|GetInstancedStaticMesh) _array_element true)))

(fn ClearHands
  (Components|InstancedStaticMesh|ClearInstances (Variables|Default|GetInstancedStaticMesh)))