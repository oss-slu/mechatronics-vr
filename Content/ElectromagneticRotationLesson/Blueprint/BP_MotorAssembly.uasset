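; BP_MotorAssembly is the motor in an electromagnetic rotation lesson, spinning once both of its contacts are connected.
; Each Tick it checks that the snap points on both contacts are assembled, then calls Spin to add local pitch rotation to the stator.
; The spin direction follows polarity: it reverses depending on whether the first contact's connected snap point is the battery's positive terminal.
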(event EventBeginPlay)

(event Collision|EventActorBeginOverlap
  (params (OtherActor :type Actor%20Object%20Reference)))

(event EventTick
  (params (DeltaSeconds :type Float%20%28single-precision%29))
  (bind _contact (Variables|Default|GetContact))
  (bind _contactsnappoint (Variables|/Game/ElectromagneticRotationLesson/Blueprint/BP_ContactPart.BP_ContactPart_C|GetContactSnapPoint _contact))
  (if (and (Variables|/Script/MechatronicsVR.SnapPointComponent|GetbIsAssembled _contactsnappoint) (Variables|/Script/MechatronicsVR.SnapPointComponent|GetbIsAssembled (Variables|/Game/ElectromagneticRotationLesson/Blueprint/BP_ContactPart2.BP_ContactPart2_C|GetContactSnapPoint (Variables|Default|GetContact2))))
    (CallFunction|Spin (Math|Float|SelectFloat 1e+01 -1e+01 (Utilities|Name|Equal(Name) (Variables|/Script/MechatronicsVR.SnapPointComponent|GetSnapID (Variables|/Script/MechatronicsVR.SnapPointComponent|GetConnectedSnapPoint _contactsnappoint)) "BatteryPositiveTerminal")))))

(fn ConstructionScript)

(fn Spin
  (params (Speed :type Float%20%28double-precision%29))
  (Transformation|AddLocalRotation (Variables|Default|GetBP_Stator) (Math|Rotator|MakeRotator 0.0 Speed 0.0) false false))