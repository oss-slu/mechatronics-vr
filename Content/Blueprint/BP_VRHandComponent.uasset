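; A VR hand component that reads XR hand tracking data and converts it into per-joint transforms.
; GetJointTransforms takes world-space tracking state for a given hand, checks that it is valid with 26 key locations and rotations, then builds an array of uniformly downscaled transforms.
; Tick calls it for the left hand only and does not use the returned array.
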(event EventBeginPlay)

(event EventTick
  (params (DeltaSeconds :type Float%20%28single-precision%29))
  (CallFunction|GetJointTransforms "Left"))

(fn GetJointTransforms
  (params (Hand :type EControllerHand%20Enum :default "Left"))
  (bind _newlocalvar (LocalVariables|GetNewLocalVar))
  ;[0 0 0 0.5] Get Actual Hand Tracking Data
  (bind _handtrackingstate (Class|HeadMountedDisplayFunctionLibrary|GetHandTrackingState 0 "UnrealWorldSpace" Hand))
  ;[0.3265 1 0 0.5] Hand Data Validaiton
  (if (.bValid (Utilities|Struct|BreakXRHandTrackingState _handtrackingstate))
    (if (and (== (Utilities|Array|Length (.HandKeyLocations (Utilities|Struct|BreakXRHandTrackingState _handtrackingstate))) 26) (== (Utilities|Array|Length (.HandKeyRotations (Utilities|Struct|BreakXRHandTrackingState _handtrackingstate))) 26))
      ;[0.006052 0.005809 0.15 0.5] Create a joint transform from the join locationsand rotationss
      (for (_ _array_index) (.HandKeyLocations (Utilities|Struct|BreakXRHandTrackingState _handtrackingstate))
        (Utilities|Array|Add _newlocalvar (Math|Transform|MakeTransform (Utilities|Array|Get(acopy) (.HandKeyLocations (Utilities|Struct|BreakXRHandTrackingState _handtrackingstate)) _array_index) (Class|KismetMathLibrary|QuatRotator (Utilities|Array|Get(acopy) (.HandKeyRotations (Utilities|Struct|BreakXRHandTrackingState _handtrackingstate)) _array_index)) "0.010000,0.010000,0.010000")))
      (return _newlocalvar))))