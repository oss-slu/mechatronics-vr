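; Quiz board actor that displays a lesson's quiz questions, choices and final score as in-world text.
; On BeginPlay, after a delay, it gets the LessonManager from MechatronicsGameMode, then finds and resets the quiz step.
; Tick polls that step while current, refreshing text when the question changes and shrinking longer questions.
; Grab components and debug keys submit answers A–D by index; the option overlap events are empty.
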(event OnComponentBeginOverlap(OptionA_C)
  (params (OverlappedComponent :type Primitive%20Component%20Object%20Reference) (OtherActor :type Actor%20Object%20Reference) (OtherComp :type Primitive%20Component%20Object%20Reference) (OtherBodyIndex :type Integer) (bFromSweep :type Boolean) (SweepResult :type Hit%20Result%20Structure%20%28by%20ref%29))
  ;[0.15 0.15 0.15 0.5] Handles input
)

(event OnComponentBeginOverlap(OptionB_C)
  (params (OverlappedComponent :type Primitive%20Component%20Object%20Reference) (OtherActor :type Actor%20Object%20Reference) (OtherComp :type Primitive%20Component%20Object%20Reference) (OtherBodyIndex :type Integer) (bFromSweep :type Boolean) (SweepResult :type Hit%20Result%20Structure%20%28by%20ref%29))
  ;[0.15 0.15 0.15 0.5] Handles input
)

(event OnComponentBeginOverlap(OptionC_C)
  (params (OverlappedComponent :type Primitive%20Component%20Object%20Reference) (OtherActor :type Actor%20Object%20Reference) (OtherComp :type Primitive%20Component%20Object%20Reference) (OtherBodyIndex :type Integer) (bFromSweep :type Boolean) (SweepResult :type Hit%20Result%20Structure%20%28by%20ref%29))
  ;[0.15 0.15 0.15 0.5] Handles input
)

(event OnComponentBeginOverlap(OptionD_C)
  (params (OverlappedComponent :type Primitive%20Component%20Object%20Reference) (OtherActor :type Actor%20Object%20Reference) (OtherComp :type Primitive%20Component%20Object%20Reference) (OtherBodyIndex :type Integer) (bFromSweep :type Boolean) (SweepResult :type Hit%20Result%20Structure%20%28by%20ref%29))
  ;[0.15 0.15 0.15 0.5] Handles input
)

(event Custom|SelectAnswerByGrip
  (params (ChoiceIndex :type Integer))
  (bind _quizlessonstep (Variables|Default|GetQuizLessonStep))
  ;[0.15 0.15 0.15 0.5] Handles input
  (Utilities|IsValid _quizlessonstep
    (:Is%20Valid
      (Class|QuizLessonStep|SubmitAnswer _quizlessonstep ChoiceIndex))))

(event Custom|SelectAnswerFromGrabComponent
  (params (SelectedGrab :type Grab%20Component%20Object%20Reference))
  (bind _grab_optiona (Variables|Default|GetGrab_OptionA))
  (bind _grab_optionb (Variables|Default|GetGrab_OptionB))
  (bind _grab_optiond (Variables|Default|GetGrab_OptionD))
  (bind _grab_optionc (Variables|Default|GetGrab_OptionC))
  (bind _array (Utilities|Array|MakeArray _grab_optiona _grab_optionb _grab_optionc _grab_optiond))
  (bind _returnvalue (Utilities|Array|FindItem _array SelectedGrab))
  ;[0.15 0.15 0.15 0.5] Handles input
  (if (>= _returnvalue 0)
    (CallFunction|SelectAnswerbyGrip _returnvalue)))

(event EventTick
  (params (DeltaSeconds :type Float%20%28single-precision%29))
  (bind _lessonmanager (Variables|Components|GetLessonManager))
  (bind _quizlessonstep (Variables|Default|GetQuizLessonStep))
  (bind _quizlessonstep_2 (Variables|Default|GetQuizLessonStep))
  (bind _returnvalue (Class|QuizLessonStep|GetCurrentQuestion _quizlessonstep_2))
  (bind (_questiontext _choices) (Utilities|Struct|BreakQuizQuestion _returnvalue))
  ;[0.15 0.15 0.15 0.5] Checks to see if the lesson step is active and what to display
  (Utilities|IsValid _lessonmanager
    (:Is%20Valid
      (Utilities|IsValid _quizlessonstep
        (:Is%20Valid
          (if (== _quizlessonstep (Class|LessonManagerComponent|GetCurrentStep _lessonmanager))
            (if (Utilities|Enum|Equal(Enum) (Variables|/Script/MechatronicsVR.QuizLessonStep|GetQuizState (Variables|Default|GetQuizLessonStep)) "ShowingResults")
              ;[0.15 0.15 0.15 0.5] Shows score
              (Rendering|Components|TextRender|SetText (Variables|Components|GetQuiz%20Question) (Utilities|Text|ToText(String) "Score:"))
              (Rendering|Components|TextRender|SetText (Variables|Components|GetAnswers) (Utilities|Text|ToText(String) (Utilities|String|Append (Utilities|String|ToString(Integer) (Variables|/Script/MechatronicsVR.QuizLessonStep|GetScore (Variables|Default|GetQuizLessonStep))) "/" (Utilities|String|ToString(Integer) (Class|QuizLessonStep|GetTotalQuestions (Variables|Default|GetQuizLessonStep))))))
              (else
                ;[0.15 0.15 0.15 0.5] Shows questions
                (Variables|/Script/MechatronicsVR.QuizLessonStep|SetQuizState (Variables|Default|GetQuizLessonStep) "ShowingQuestion")
                (if (Utilities|Enum|NotEqual(Enum) _questiontext (Variables|Default|GetCurrentQuizQuestion))
                  (CallFunction|SetQuestionText _questiontext _choices))))))))))

(event EventBeginPlay
  ;[0.15 0.15 0.15 0.5] This entire thing is to find the Lesson manager and get the lesson step in order to eventually display quiz stuff
  (Utilities|FlowControl|Delay 1.0)
  (bind _outactors (Actor|GetAllActorsOfClass "/Script/MechatronicsVR.LessonUIActor"))
  (Variables|Default|SetLessonUIActor (Utilities|Array|Get(acopy) _outactors))
  (bind _asmechatronics_game_mode (Utilities|Casting|CastToMechatronicsGameMode (Game|GetGameMode))
    (:then
      (bind _output_get (Variables|Components|SetLessonManager (Variables|/Script/MechatronicsVR.MechatronicsGameMode|GetLessonManager _asmechatronics_game_mode)))
      (Development|PrintText "Got Mechatronics Game mode")
      (Development|PrintString (Utilities|String|ToString(Integer) (Utilities|Array|Length (Variables|/Script/MechatronicsVR.LessonManagerComponent|GetLessonSteps _output_get))))
      (for _array_element (Variables|/Script/MechatronicsVR.LessonManagerComponent|GetLessonSteps _output_get)
        (Development|PrintString (Utilities|String|EnumtoString (Variables|/Script/MechatronicsVR.LessonStep|GetStepType _array_element)))
        (if (Utilities|Enum|Equal(Enum) (Variables|/Script/MechatronicsVR.LessonStep|GetStepType _array_element) "Quiz")
          (bind _asquiz_lesson_step (Utilities|Casting|CastToQuizLessonStep _array_element))
          (Variables|Default|SetQuizLessonStep _asquiz_lesson_step)
          (Development|PrintText "SetQuizStep")
          (Class|LessonStep|ResetStep (Variables|Default|GetQuizLessonStep))))
      (Development|PrintText "Done looking for steps"))
    (:CastFailed
      (Development|PrintText "failed to find mechatronics game mode"))))

(event Input|KeyboardEvents|DebugKeyA
  (params (Key :type Key%20Structure :default "None") (ActionValue :type Input%20Action%20Value%20Structure))
  ;[0.15 0.15 0.15 0.5] Handles input
  (:Pressed
    (Development|PrintText "DEBUG: Selected A")
    (Class|QuizLessonStep|SubmitAnswer (Variables|Default|GetQuizLessonStep))))

(event Input|KeyboardEvents|DebugKeyB
  (params (Key :type Key%20Structure :default "None") (ActionValue :type Input%20Action%20Value%20Structure))
  ;[0.15 0.15 0.15 0.5] Handles input
  (:Pressed
    (Development|PrintText "DEBUG: Selected B")
    (Class|QuizLessonStep|SubmitAnswer (Variables|Default|GetQuizLessonStep) 1)))

(event Input|KeyboardEvents|DebugKeyC
  (params (Key :type Key%20Structure :default "None") (ActionValue :type Input%20Action%20Value%20Structure))
  ;[0.15 0.15 0.15 0.5] Handles input
  (:Pressed
    (Development|PrintText "DEBUG: Selected C")
    (Class|QuizLessonStep|SubmitAnswer (Variables|Default|GetQuizLessonStep) 2)))

(event Input|KeyboardEvents|DebugKeyD
  (params (Key :type Key%20Structure :default "None") (ActionValue :type Input%20Action%20Value%20Structure))
  ;[0.15 0.15 0.15 0.5] Handles input
  (:Pressed
    (Development|PrintText "DEBUG: Selected D")
    (Class|QuizLessonStep|SubmitAnswer (Variables|Default|GetQuizLessonStep) 3)))

(fn ConstructionScript)

(fn SetQuestionText
  (params (NewQuestion :type String) (NewAnswers :type Array%20of%20Quiz%20Choice%20Structures))
  (bind _quiz_question (Variables|Components|GetQuiz%20Question))
  (bind _output_get (Variables|Default|SetCurrentQuizQuestion NewQuestion))
  (Rendering|Components|TextRender|SetWorldSize _quiz_question (Math|Float|MapRangeClamped (Math|Conversions|ToFloat(Integer) (Utilities|String|Len _output_get)) 0.0 1e+02 15.0 6.0))
  (Rendering|Components|TextRender|SetText _quiz_question (Utilities|Text|ToText(String) _output_get))
  (Variables|Default|SetCurrentAnswerString "")
  (for (_array_element _array_index) NewAnswers
    (Variables|Default|SetCurrentAnswerString (Utilities|String|Append (Variables|Default|GetCurrentAnswerString) (Utilities|String|ToString(Integer) (+ _array_index 1)) ": " (.ChoiceText (Utilities|Struct|BreakQuizChoice _array_element)) " 
")))
  (Rendering|Components|TextRender|SetText (Variables|Components|GetAnswers) (Utilities|Text|ToText(String) (Variables|Default|GetCurrentAnswerString))))