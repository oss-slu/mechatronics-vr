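; Power supply actor that steps through preset voltages with plus and minus touch buttons to drive motorized parts.
; On BeginPlay it gathers every motorized PartActor, applies the starting preset, then runs a hardcoded, timed test sweep through six presets.
; SetVoltage feeds each motor a 0–1 speed relative to the highest preset, updates the voltage text and turns the light red at zero, green otherwise.
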(event OnInputTouchEnter(ButtonMinus)
  (params (FingerIndex :type ETouchIndex%20Enum :default "Touch1") (TouchedComponent :type Primitive%20Component%20Object%20Reference))
  ;[0.15 0.15 0.15 0.5] Logic to update vontage when hitting the minus button
  (if (!= (Variables|Default|GetCurrentVoltageIndex) 0)
    (bind _output_get (Variables|Default|SetCurrentVoltageIndex (- (Variables|Default|GetCurrentVoltageIndex) 1)))
    (bind _output_get_2 (Variables|Default|SetCurrentVoltage (Utilities|Array|Get(acopy) (Variables|Default|GetVoltagePresets) _output_get)))
    (CallFunction|SetVoltage _output_get_2)))

(event OnInputTouchEnter(ButtonPlus)
  (params (FingerIndex :type ETouchIndex%20Enum :default "Touch1") (TouchedComponent :type Primitive%20Component%20Object%20Reference))
  ;[0.15 0.15 0.15 0.5] Logic to update voltage when hitting the plus button
  (if (!= (Utilities|Array|LastIndex (Variables|Default|GetVoltagePresets)) (Variables|Default|GetCurrentVoltageIndex))
    (bind _output_get (Variables|Default|SetCurrentVoltageIndex (+ (Variables|Default|GetCurrentVoltageIndex) 1)))
    (bind _output_get_2 (Variables|Default|SetCurrentVoltage (Utilities|Array|Get(acopy) (Variables|Default|GetVoltagePresets) _output_get)))
    (CallFunction|SetVoltage _output_get_2)))

(event EventBeginPlay
  (bind _voltagepresets (Variables|Default|GetVoltagePresets))
  (Variables|Default|SetMaxVoltage (.MaxValue (Math|Float|MaxOfFloatArray (Variables|Default|GetVoltagePresets))))
  (CallFunction|FindMotor)
  (bind _output_get (Variables|Default|SetCurrentVoltage (Utilities|Array|Get(acopy) (Variables|Default|GetVoltagePresets) (Variables|Default|GetCurrentVoltageIndex))))
  (CallFunction|SetVoltage _output_get)
  (Utilities|FlowControl|Delay 2.0)
  ;[0.15 0.15 0.15 0.5] I am sorry, this is for testing, this is awful and should not exist, but for each loops do not work in unreal
  (CallFunction|TestPowerSupplySet (Utilities|Array|Get(acopy) _voltagepresets))
  (Utilities|FlowControl|Delay 1.0)
  (CallFunction|TestPowerSupplySet (Utilities|Array|Get(acopy) _voltagepresets 1))
  (Utilities|FlowControl|Delay 1.0)
  (CallFunction|TestPowerSupplySet (Utilities|Array|Get(acopy) _voltagepresets 2))
  (Utilities|FlowControl|Delay 1.0)
  (CallFunction|TestPowerSupplySet (Utilities|Array|Get(acopy) _voltagepresets 3))
  (Utilities|FlowControl|Delay 1.0)
  (CallFunction|TestPowerSupplySet (Utilities|Array|Get(acopy) _voltagepresets 4))
  (Utilities|FlowControl|Delay 1.0)
  (CallFunction|TestPowerSupplySet (Utilities|Array|Get(acopy) _voltagepresets 5)))

(event Collision|EventActorBeginOverlap
  (params (OtherActor :type Actor%20Object%20Reference)))

(event EventTick
  (params (DeltaSeconds :type Float%20%28single-precision%29)))

(fn ConstructionScript)

(fn SetVoltage
  (params (NewVoltage :type Float%20%28double-precision%29))
  (bind _onofflight (Variables|Default|GetOnOffLight))
  (if (== 0.0 NewVoltage)
    (Rendering|Components|Light|SetLightColor _onofflight "(R=1.000000,G=0.000000,B=0.000000,A=1.000000)" true)
    (else
      (Rendering|Components|Light|SetLightColor _onofflight "(R=0.000000,G=1.000000,B=0.000000,A=1.000000)" true)))
  (for _array_element (Variables|Default|GetMotor)
    (Class|PartActor|SetMotorSpeed _array_element (Math|Float|Clamp(Float) (/ NewVoltage (Variables|Default|GetMaxVoltage)))))
  (Rendering|Components|TextRender|SetText (Variables|Default|GetVoltageText) (Utilities|Text|FormatText (Utilities|Text|ToText(Float) NewVoltage "HalfToEven") 0)))

(fn FindMotor
  (bind _outactors (Actor|GetAllActorsOfClass "/Script/MechatronicsVR.PartActor"))
  (for _array_element _outactors
    (if (Variables|/Script/MechatronicsVR.PartActor|GetbIsMotorized _array_element)
      (Utilities|Array|AddUnique (Variables|Default|GetMotor) _array_element)
      (Development|PrintString "Added new motor"))))

(fn TestPowerSupplySet
  (params (NewParam :type Float%20%28double-precision%29))
  (Development|PrintString (Utilities|String|ToString(Text) (Utilities|Text|FormatText (Utilities|Text|FormatText "Set Voltage to ") (Utilities|Text|ToText(Float) NewParam "HalfToEven"))))
  (CallFunction|SetVoltage NewParam))